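; Magic system component that gates spell casting on a busy flag and available mana.
; CastMagic returns true if a cast is already active; otherwise it sets IsCasting, then compares Mana to the spell's cost.
; With enough mana it deducts the clamped cost, calls Cast with the spell and returns false.
; Insufficient mana returns true with IsCasting still set, and nothing here clears that flag.
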(event EventBeginPlay)

(event EventTick
  (params (DeltaSeconds :type Float%20%28single-precision%29)))

(fn CastMagic
  (params (Spell :type BP%20Spell%20Object%20Reference))
  (if (Variables|Default|GetIsCasting)
    (return true)
    (else
      (Variables|Default|SetIsCasting true)
      (if (>= (Variables|Default|GetMana) (Variables|/Game/Spells/BP_Spell.BP_Spell_C|GetCost Spell))
        (Variables|Default|SetMana (Math|Float|Clamp(Float) (- (Variables|Default|GetMana) (Variables|/Game/Spells/BP_Spell.BP_Spell_C|GetCost Spell)) 0.0 (Variables|Default|GetMax%20Mana)))
        (Default|CallCast Spell)
        (return false)
        (else
          (return true))))))