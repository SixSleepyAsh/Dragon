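; Damage system component that tracks an actor's health, death, blocking and invincibility.
; Heal adds health clamped to the maximum while the actor is alive.
; Hurt takes a DamageInfo and routes it through the CanBeDamage macro, where trample bypasses invincibility and blockable hits can be blocked.
; Event dispatchers report blocks with parry info, death, and damage responses when the actor is interruptable or the hit forces an interrupt.
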(event EventBeginPlay)

(event EventTick
  (params (DeltaSeconds :type Float%20%28single-precision%29)))

(fn Heal
  (params (Amount :type Float%20%28double-precision%29))
  (if (not (Variables|Default|GetisDead))
    (bind _output_get (Variables|Default|SetHealth (Math|Float|Clamp(Float) (+ (Variables|Default|GetHealth) (Math|Float|Absolute(Float) Amount)) 0.0 (Variables|Default|GetMaxHealth))))
    (return _output_get)))

(fn Hurt
  (params (DamageInfo :type BPS%20Damage%20Info%20Structure))
  (Utilities|CanbeDamage (.trample DamageInfo) (.blockable DamageInfo)
    (:BlockDamage
      (Default|CallOnBlock (.parriable DamageInfo))
      (return false))
    (:Damage
      (bind _output_get (Variables|Default|SetHealth (- (Variables|Default|GetHealth) (.amount DamageInfo))))
      (if (<= _output_get 0.0)
        (Variables|Default|SetisDead true)
        (Default|CallOnDeath)
        (return true)
        (elif (or (Variables|Default|GetisInterruptable) (.interrupt DamageInfo))
          (Default|CallOnDamageResponse (.damageresponse DamageInfo))
          (return true))))
    (:NoDamge
      (return false))))